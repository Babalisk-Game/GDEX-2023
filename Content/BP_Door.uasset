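; BP_Door is an interactive door that swings open with sound, stops blocking pawns, and can be slammed shut instantly.
; TryOpen reopens player-closed doors directly, otherwise flashes blue and shows the opener's door widget, which hides when the player's overlap ends.
; Overlapping BP_Indoor actors receive the door through OpenDoor.
; Tick interpolates toward the desired rotation, snapping within a forward-vector tolerance, while a Mimicry timeline can also drive that rotation.
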(event `self.ReceiveTick`
  (params (DeltaSeconds :type "Float (single-precision)"))
  (if (`self.Opening?`)
    (`self.K2_SetActorRotation` (`KismetMathLibrary.RInterpTo` (`self.K2_GetActorRotation`) (`self.DesiredRotation`) DeltaSeconds 1.0))
    ;[1 1 1] Is Door Opened?
    (bind _output_get (set `self.Opened?` (`KismetMathLibrary.Vector_IsNearlyZero` (- (`KismetMathLibrary.GetForwardVector` (`self.DesiredRotation`)) (`KismetMathLibrary.GetForwardVector` (`self.K2_GetActorRotation`))) 0.4)))
    (if _output_get
      (set `self.Opening?` false)
      (`self.K2_SetActorRotation` (`self.DesiredRotation`)))))

(event `self.Interaction.OnComponentBeginOverlap`
  (params (OverlappedComponent :type "PrimitiveComponent Object Reference") (OtherActor :type "Actor Object Reference") (OtherComp :type "PrimitiveComponent Object Reference") (OtherBodyIndex :type Integer) (bFromSweep :type Boolean) (SweepResult :type "HitResult Structure (by ref)"))
  (`|ExecutionSequence`
    (:`then_0`
      (if (not (or (`self.Opened?`) (`self.Opening?`)))
        ;[1 1 1] Closed Door
        (if (`self.ClosedByPlayer?`)
          _)))
    (:`then_1`
      ;[1 1 1] Indoor Opening
      (bind _asbp_indoor (cast `/Game/FirstPerson/Blueprints/BP_Indoor` OtherActor))
      (`/Game/FirstPerson/Blueprints/BP_Indoor.OpenDoor` _asbp_indoor self false))))

(event `Mimicry`
  ;[1 1 1] Mimic
  (bind (_direction _newtrack_0) (`Timeline|Timeline` :!via `PlayFromStart`)
    (:`Update`
      (set `self.Opening?` true)
      (set `self.DesiredRotation` (`KismetMathLibrary.MakeRotFromZ` _newtrack_0))
      (set `self.Interactable?` false))))

(event `self.Interaction.OnComponentEndOverlap`
  (params (OverlappedComponent :type "PrimitiveComponent Object Reference") (OtherActor :type "Actor Object Reference") (OtherComp :type "PrimitiveComponent Object Reference") (OtherBodyIndex :type Integer))
  (bind _asbp_first_person_character (cast `/Game/FirstPerson/Blueprints/BP_FirstPersonCharacter` OtherActor))
  (`/Game/FirstPerson/Blueprints/BP_FirstPersonCharacter.Close Door Widget` _asbp_first_person_character)
  (`self.PlayerDoneInteracting`))

(event `PlayerInteracting`
  (`PrimitiveComponent.SetMaterial` (`self.StaticMesh`) 0 "/Game/LevelPrototyping/Materials/MI_Solid_Blue.MI_Solid_Blue")
  (`KismetSystemLibrary.Delay` 0.2)
  (`self.PlayerDoneInteracting`))

(event `PlayerDoneInteracting`
  (`PrimitiveComponent.SetMaterial` (`self.StaticMesh`) 0 "/Game/StarterContent/Props/Materials/M_Door.M_Door"))

(fn `Close`
  (if (`self.Opened?`)
    (`PrimitiveComponent.SetCollisionResponseToChannel` (`self.StaticMesh`) "ECC_Pawn" "ECR_Block")
    (`self.K2_SetActorRotation` (`self.InitialRotation`))
    (set `self.ClosedByPlayer?` true)
    (set `self.Opened?` false)
    ;[1 1 1] Audio
    (`GameplayStatics.PlaySoundAtLocation` "/Game/Sounds/doorslam-shortened.doorslam-shortened" (`self.K2_GetActorLocation`) (struct) 1.0 (`KismetMathLibrary.RandomFloatInRange` 0.8 1.0) (`KismetMathLibrary.RandomFloatInRange` 0.0 0.5) null null null null)))

(fn `Open`
  (`self.PlayerDoneInteracting`)
  (set `self.Opening?` true)
  (set `self.DesiredRotation` (`KismetMathLibrary.ComposeRotators` (`self.InitialRotation`) (struct :`Yaw` 90.0)))
  (set `self.Interactable?` false)
  ;[1 1 1] Collision for player and orb
  (`PrimitiveComponent.SetCollisionResponseToChannel` (`self.StaticMesh`) "ECC_Pawn" "ECR_Ignore")
  ;[1 1 1] Audio
  (`GameplayStatics.PlaySoundAtLocation` "/Game/Sounds/door-2-6841.door-2-6841" (`self.K2_GetActorLocation`) (struct) 1.0 (`KismetMathLibrary.RandomFloatInRange` 0.8 1.0) (`KismetMathLibrary.RandomFloatInRange` 0.0 0.5) null null null null))

(fn `TryOpen`
  (params (Opener :type "/Game/FirstPerson/Blueprints/BP_FirstPersonCharacter Object Reference"))
  (if (or (`self.Opened?`) (`self.Opening?`))
    (`KismetSystemLibrary.PrintString` "No interact. Door is moving")
    (elif (`self.ClosedByPlayer?`)
      (`self.Open`)
      (else
        (`self.PlayerInteracting`)
        (`/Game/FirstPerson/Blueprints/BP_FirstPersonCharacter.Open Door Widget` Opener self)))))

(fn `UserConstructionScript`
  (`|ExecutionSequence`
    (:`then_0`
      (`PrimitiveComponent.SetMaterial` (`self.StaticMesh`) 0 (`/Game/BP_DoorData.StaticMesh` (`self.Data`))))
    (:`then_1`
      (set `self.InitialRotation` (`self.K2_GetActorRotation`)))
    (:`then_2`
      (if (`self.UseLongCollisionDepth?`)
        (`BoxComponent.SetBoxExtent` (`self.Interaction`) (64.0 48.0 64.0) true)))))